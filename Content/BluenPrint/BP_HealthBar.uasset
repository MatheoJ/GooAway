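; Health bar actor that displays the remaining life of an objective using the Health and Health1 components.
; LifeIsUpdated maps current life from a 100-point range to the relative Z scale of Health, so the bar shrinks as life drops.
; ObjectiveDead turns off custom depth rendering on both components.
; An inverse scaling of Health1 is present but unconnected, so only Health resizes.
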(event EventBeginPlay)

(event Collision|EventActorBeginOverlap
  (params (OtherActor :type Actor%20Object%20Reference)))

(event EventTick
  (params (DeltaSeconds :type Float%20%28single-precision%29)))

(event EventLifeIsUpdated
  (params (CurrentLife :type Float%20%28double-precision%29))
  (bind _health (Variables|Default|GetHealth))
  (bind _relativescale3d (Variables|/Script/Engine.SceneComponent|GetRelativeScale3D _health))
  (Transformation|SetRelativeScale3D _health (Math|Vector|MakeVector (.x _relativescale3d) (.y _relativescale3d) (Math|Float|Lerp 1.0 0.0 (Math|Float|MapRangeClamped CurrentLife 1e+02 0.0 0.0 1.0)))))

(event EventObjectiveDead
  (Rendering|SetRenderCustomDepth (Variables|Default|GetHealth1) false)
  (Rendering|SetRenderCustomDepth (Variables|Default|GetHealth) false))

(fn ConstructionScript)