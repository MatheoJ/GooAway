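; BP_OilSpill is an oil puddle that ignites when an Electric slime overlaps it and evaporates Water slimes with an effect, destroying them.
; Its fire Niagara effect stays paused until SetOnFire runs.
; Ignition sphere-overlaps nearby oil spills, flags unlit ones as burning and schedules their SetOnFire with a delay scaled by distance, producing a spreading chain reaction.
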(event EventBeginPlay
  (Class|NiagaraComponent|SetPaused (Variables|Default|GetNS_fire) true))

(event Collision|EventActorBeginOverlap
  (params (OtherActor :type Actor%20Object%20Reference))
  (bind _asslime_base (Utilities|Casting|CastToSlimeBase OtherActor))
  (switch Utilities|FlowControl|Switch|SwitchonESlimeType (Variables|/Script/Pompastronautes.SlimeBase|GetSlimeType _asslime_base)
    (:Water
      (Niagara|SpawnSystematLocation (Variables|Default|GetEvaporationFX) (Transformation|GetActorLocation _asslime_base))
      (Actor|DestroyActor _asslime_base))
    (:Electric
      (if (not (Variables|Default|GetIsOnFire))
        (CallFunction|SetonFire)))))

(event EventTick
  (params (DeltaSeconds :type Float%20%28single-precision%29)))

(fn ConstructionScript)

(fn SetonFire
  (Variables|Default|SetIsOnFire true)
  (Class|NiagaraComponent|SetPaused (Variables|Default|GetNS_fire) false)
  (bind _outactors (Collision|SphereOverlapActors (Transformation|GetActorLocation) (Variables|Default|GetFlamableRadius) (Utilities|Array|MakeArray (Variables|Default|GetObjectType)) "BP_OilSpill_C"))
  (Development|PrintString (Utilities|String|ToString(Integer) (Utilities|Array|Length _outactors)))
  (for _array_element _outactors
    (bind _asbp_oil_spill (Utilities|Casting|CastToBP_OilSpill _array_element))
    (if (not (Variables|BP_OilSpill_C|GetIsOnFire _asbp_oil_spill))
      (Variables|BP_OilSpill_C|SetIsOnFire _asbp_oil_spill true)
      (Utilities|Time|SetTimerbyFunctionName _asbp_oil_spill "SetOnFire" (Math|Float|Lerp (Variables|Default|GetMinFlamableDelay) (Variables|Default|GetMaxFlamableDelay) (/ (Math|Vector|Distance(Vector) (Transformation|GetActorLocation _asbp_oil_spill) (Transformation|GetActorLocation)) (Variables|Default|GetFlamableRadius)))))))