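; BP_LevelTimer is an actor that displays the level's remaining time as text in the world.
; On BeginPlay it caches a reference to the GM_Pompastronautes game mode, which holds the countdown value.
; Every Tick it reads CurrentRemainingTime, rounds it and writes it to its TextRender component as a labeled seconds readout.
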(event EventBeginPlay
  (bind _asgm_pompastronautes (Utilities|Casting|CastToGM_Pompastronautes (Game|GetGameMode)))
  (Variables|Default|SetAs%20GM%20Pompastronautes _asgm_pompastronautes))

(event Collision|EventActorBeginOverlap
  (params (OtherActor :type Actor%20Object%20Reference)))

(event EventTick
  (params (DeltaSeconds :type Float%20%28single-precision%29))
  (Rendering|Components|TextRender|SetText (Variables|Default|GetTextRender) (Utilities|Text|ToText(String) (Utilities|String|Append "Timer : " (Utilities|String|ToString(Integer) (Math|Float|Round (Variables|/Game/BluenPrint/GM_Pompastronautes.GM_Pompastronautes_C|GetCurrentRemainingTime (Variables|Default|GetAs%20GM%20Pompastronautes)))) "s"))))

(fn ConstructionScript)