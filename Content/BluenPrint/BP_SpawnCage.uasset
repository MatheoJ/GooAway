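; BP_SpawnCage is a slime spawner that keeps replenishing a Water, Electric or Oil slime pawn, chosen by an enum.
; It spawns one at SpawnPoint on BeginPlay, flagged NotMooving, and tracks it as LastSlimeSpawned.
; When that slime stops overlapping the cage, the reference clears and a timer calls SpawnSlime again after SpawnDelay.
; If CanMove is false, the new slime's Instigator is detached from its controller.
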(event EventBeginPlay
  (CallFunction|SpawnSlime))

(event Collision|EventActorBeginOverlap
  (params (OtherActor :type Actor%20Object%20Reference)))

(event EventTick
  (params (DeltaSeconds :type Float%20%28single-precision%29)))

(event Collision|EventActorEndOverlap
  (params (OtherActor :type Actor%20Object%20Reference))
  (if (== OtherActor (Variables|Default|GetLastSlimeSpawned))
    (Variables|Default|SetLastSlimeSpawned 0)
    (Utilities|Time|SetTimerbyFunctionName 0 "SpawnSlime" (Variables|Default|GetSpawnDelay))))

(fn ConstructionScript)

(fn SpawnSlime
  (switch Utilities|FlowControl|Switch|SwitchonESlimeType (Variables|Default|Getenum)
    (:Water
      (bind _returnvalue (Game|SpawnActorfromClass "/Game/BluenPrint/Slime/BP_WaterSlimePawn.BP_WaterSlimePawn_C" (Math|Transform|MakeTransform (Transformation|GetWorldLocation (Variables|Default|GetSpawnPoint)) "0, 0, 0" "1.000000,1.000000,1.000000") "AdjustIfPossibleButAlwaysSpawn" "MultiplyWithRoot" 0 true 0))
      (Variables|Default|SetLastSlimeSpawned _returnvalue)
      (if (not (Variables|Default|GetCanMove))
        (Class|Pawn|DetachfromControllerPendingDestroy (Variables|/Script/Engine.Actor|GetInstigator _returnvalue))))
    (:Electric
      (bind _returnvalue_2 (Game|SpawnActorfromClass "/Game/BluenPrint/Slime/BP_ElectricSlimePawn.BP_ElectricSlimePawn_C" (Math|Transform|MakeTransform (Transformation|GetWorldLocation (Variables|Default|GetSpawnPoint)) "0, 0, 0" "1.000000,1.000000,1.000000") "AdjustIfPossibleButAlwaysSpawn" "MultiplyWithRoot" 0 true 0))
      (Variables|Default|SetLastSlimeSpawned _returnvalue_2)
      (if (not (Variables|Default|GetCanMove))
        (Class|Pawn|DetachfromControllerPendingDestroy (Variables|/Script/Engine.Actor|GetInstigator _returnvalue_2))))
    (:Oil
      (bind _returnvalue_3 (Game|SpawnActorfromClass "/Game/BluenPrint/Slime/BP_OilSlimePawn.BP_OilSlimePawn_C" (Math|Transform|MakeTransform (Transformation|GetWorldLocation (Variables|Default|GetSpawnPoint)) "0, 0, 0" "1.000000,1.000000,1.000000") "AdjustIfPossibleButAlwaysSpawn" "MultiplyWithRoot" 0 true 0))
      (Variables|Default|SetLastSlimeSpawned _returnvalue_3)
      (if (not (Variables|Default|GetCanMove))
        (Class|Pawn|DetachfromControllerPendingDestroy (Variables|/Script/Engine.Actor|GetInstigator _returnvalue_3))))))