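; Level-transition manager that streams neighboring levels in and out as players cross its Load and Unload trigger volumes.
; Each trigger toggles characters in a passed-players list, acting when a second player is added, or any in solo mode.
; Load streams in the next level, refreshes HUD health bars, then opens the next doors after a delay.
; Unload permanently closes the previous doors, unloads that level and destroys all SlimeBase actors.
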(event OnComponentBeginOverlap(Unload)
  (params (OverlappedComponent :type Primitive%20Component%20Object%20Reference) (OtherActor :type Actor%20Object%20Reference) (OtherComp :type Primitive%20Component%20Object%20Reference) (OtherBodyIndex :type Integer) (bFromSweep :type Boolean) (SweepResult :type Hit%20Result%20Structure%20%28by%20ref%29))
  (bind _passedplayersunload (Variables|Default|GetPassedPlayersUnload))
  (bind _previousdoubledoors (Variables|Default|GetPreviousDoubleDoors))
  (bind _asbp_third_person_character_only_bp (Utilities|Casting|CastToBP_ThirdPersonCharacter_onlyBP OtherActor))
  (if (Utilities|Array|ContainsItem _passedplayersunload _asbp_third_person_character_only_bp)
    (Utilities|Array|RemoveItem _passedplayersunload _asbp_third_person_character_only_bp)
    (else
      (Utilities|Array|Add _passedplayersunload _asbp_third_person_character_only_bp)
      (if (or (> (Utilities|Array|Length (Variables|Default|GetPassedPlayersUnload)) 1) (Variables|Default|GetsoloPlayer))
        (Default|CloseDoors _previousdoubledoors)
        (Variables|/Game/LevelPrototyping/DymanicObjects/BP_DoubleDoors.BP_DoubleDoors_C|SetclosedForever _previousdoubledoors true)
        (Game|UnloadStreamLevel(byName) (Variables|Default|GetNamePreviousLvl) false)
        (bind _outactors (Actor|GetAllActorsOfClass "/Script/Pompastronautes.SlimeBase"))
        (for _array_element _outactors
          (Actor|DestroyActor _array_element))))))

(event OnComponentBeginOverlap(Load)
  (params (OverlappedComponent :type Primitive%20Component%20Object%20Reference) (OtherActor :type Actor%20Object%20Reference) (OtherComp :type Primitive%20Component%20Object%20Reference) (OtherBodyIndex :type Integer) (bFromSweep :type Boolean) (SweepResult :type Hit%20Result%20Structure%20%28by%20ref%29))
  (bind _passedplayersload (Variables|Default|GetPassedPlayersLoad))
  (bind _asbp_third_person_character_only_bp (Utilities|Casting|CastToBP_ThirdPersonCharacter_onlyBP OtherActor))
  (if (Utilities|Array|ContainsItem _passedplayersload _asbp_third_person_character_only_bp)
    (Utilities|Array|RemoveItem _passedplayersload _asbp_third_person_character_only_bp)
    (else
      (Utilities|Array|Add _passedplayersload _asbp_third_person_character_only_bp)
      (if (or (> (Utilities|Array|Length (Variables|Default|GetPassedPlayersLoad)) 1) (Variables|Default|GetsoloPlayer))
        (Game|LoadStreamLevel(byName) (Variables|Default|GetNameNextLvl) true)
        (bind _foundwidgets (Widget|GetAllWidgetsOfClass "/Game/Widgets/WB_HUD.WB_HUD_C" true))
        (Default|UpdateHealthBars (Utilities|Array|Get(acopy) _foundwidgets (Utilities|Array|LastIndex _foundwidgets)))
        (Utilities|FlowControl|Delay (Variables|Default|GetDelaiAvantOuverturePortes))
        (Default|SlideDoorsEvent (Variables|Default|GetNextDoubleDoors))))))

(event EventBeginPlay
  (Variables|/Game/LevelPrototyping/DymanicObjects/BP_DoubleDoors.BP_DoubleDoors_C|SetOpenByLoadManager (Variables|Default|GetNextDoubleDoors) true))

(event Collision|EventActorBeginOverlap
  (params (OtherActor :type Actor%20Object%20Reference)))

(event EventTick
  (params (DeltaSeconds :type Float%20%28single-precision%29)))

(fn ConstructionScript)