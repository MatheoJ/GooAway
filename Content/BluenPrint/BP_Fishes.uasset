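; BP_Fishes is a decorative fish group that circles on two pivots and stays below a given surface height.
; Tick spins the two pivots slowly in opposite directions by a fixed step per frame, independent of delta time.
; FishUpdate lowers any descendant component of the root at or above the supplied surface Z to that height.
; ObjectiveDead hides the group by scaling every descendant component to zero.
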(event EventObjectiveDead
  (for _array_element (Components|GetChildrenComponents (Variables|Default|GetDefaultSceneRoot) true)
    (Transformation|SetRelativeScale3D _array_element "0, 0, 0")))

(event EventFishUpdate
  (params (surface :type Vector :default "0, 0, 0"))
  (bind _z (Math|Vector|BreakVector surface))
  (for _array_element (Components|GetChildrenComponents (Variables|Default|GetDefaultSceneRoot) true)
    (if (<= _z (.z (Transformation|GetWorldLocation _array_element)))
      (Transformation|SetWorldLocation _array_element (Math|Vector|MakeVector (.x (Transformation|GetWorldLocation _array_element)) (.y (Transformation|GetWorldLocation _array_element)) _z) false false))))

(event EventTick
  (params (DeltaSeconds :type Float%20%28single-precision%29))
  (Transformation|AddLocalRotation (Variables|Default|Getpivot) "0.000000,0.600000,0.000000" false false)
  (Transformation|AddLocalRotation (Variables|Default|Getpivot2) "0.000000,-0.500000,0.000000" false false))

(fn ConstructionScript)