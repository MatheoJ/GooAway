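; Radio actor that starts audio playback through one-shot gates fed by Sphere overlap and pause changes, and enables physics on its mesh on first Box overlap.
; Tick watches pause state, switching the audio to UI sound and resuming from a tracked position when paused, then clearing that flag on unpause.
; A looping timer advances the tracked position, wrapping at the sound's duration.
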(event OnComponentBeginOverlap(Sphere)
  (params (OverlappedComponent :type Primitive%20Component%20Object%20Reference) (OtherActor :type Actor%20Object%20Reference) (OtherComp :type Primitive%20Component%20Object%20Reference) (OtherBodyIndex :type Integer) (bFromSweep :type Boolean) (SweepResult :type Hit%20Result%20Structure%20%28by%20ref%29))
  (Utilities|FlowControl|DoOnce false
    (:Completed
      (Utilities|FlowControl|DoOnce false
        (:Completed
          (Utilities|FlowControl|Sequence
            (:then_0
              (Utilities|FlowControl|DoOnce false
                (:Completed
                  (Audio|Components|Audio|Play (Variables|Default|GetAudio) 0.0)
                  (bind _returnvalue (Utilities|Time|SetTimerbyEvent (delegate Custom|TimerV) 0.1 true)))))))))))

(event OnComponentBeginOverlap(Box)
  (params (OverlappedComponent :type Primitive%20Component%20Object%20Reference) (OtherActor :type Actor%20Object%20Reference) (OtherComp :type Primitive%20Component%20Object%20Reference) (OtherBodyIndex :type Integer) (bFromSweep :type Boolean) (SweepResult :type Hit%20Result%20Structure%20%28by%20ref%29))
  (Utilities|FlowControl|DoOnce false
    (:Completed
      (Physics|SetSimulatePhysics (Variables|Default|Getradio) true))))

(event Custom|TimerV
  (CallFunction|Timec (Variables|/Script/Engine.SoundBase|GetDuration (Variables|/Script/Engine.AudioComponent|GetSound (Variables|Default|GetAudio)))))

(event EventBeginPlay)

(event Collision|EventActorBeginOverlap
  (params (OtherActor :type Actor%20Object%20Reference)))

(event EventTick
  (params (DeltaSeconds :type Float%20%28single-precision%29))
  (bind _audio (Variables|Default|GetAudio))
  (if (Game|IsGamePaused)
    (Utilities|FlowControl|DoOnce false :!label _label
      (:Completed
        (Class|AudioComponent|SetUISound _audio true)
        (Audio|Components|Audio|Play (Variables|Default|GetAudio) (Variables|Default|GetTimeEllapsed))
        (Utilities|FlowControl|Sequence
          (:then_0
            (goto _label_2 Reset))
          (:then_1
            (goto _label_3 Reset)))))
    (else
      (Utilities|FlowControl|Sequence
        (:then_0
          (goto _label Reset))
        (:then_1
          (Utilities|FlowControl|DoOnce true :!label _label_2
            (:Completed
              (Class|AudioComponent|SetUISound _audio false)
              (Utilities|FlowControl|DoOnce false :!label _label_3
                (:Completed
                  (Utilities|FlowControl|Sequence
                    (:then_0
                      (Utilities|FlowControl|DoOnce false
                        (:Completed
                          (Audio|Components|Audio|Play (Variables|Default|GetAudio) 0.0)
                          (bind _returnvalue (Utilities|Time|SetTimerbyEvent (delegate Custom|TimerV) 0.1 true)))))))))))))))

(fn ConstructionScript)

(fn Timec
  (params (duration :type Float%20%28double-precision%29))
  (if (> duration (Variables|Default|GetTimeEllapsed))
    (Variables|Default|SetTimeEllapsed (+ (Variables|Default|GetTimeEllapsed) 0.2))
    (else
      (Variables|Default|SetTimeEllapsed 0.0)))
  (return))