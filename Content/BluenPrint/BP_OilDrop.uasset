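; BP_OilDrop is an oil droplet actor that leaves an oil spill where it hits a surface.
; On hit it spawns a BP_OilSpill at the impact point, oriented to the surface normal, then destroys itself.
; Its fire Niagara effect starts paused; SetonFire unpauses it and sets IsOnFire, so a burning drop ignites the spill it spawns.
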(event EventBeginPlay
  (Class|NiagaraComponent|SetPaused (Variables|Default|GetNS_fire) true))

(event EventSetonFire
  (Class|NiagaraComponent|SetPaused (Variables|Default|GetNS_fire) false)
  (Variables|Default|SetIsOnFire true))

(event EventTick
  (params (DeltaSeconds :type Float%20%28single-precision%29)))

(event Collision|EventHit
  (params (MyComp :type Primitive%20Component%20Object%20Reference) (Other :type Actor%20Object%20Reference) (OtherComp :type Primitive%20Component%20Object%20Reference) (bSelfMoved :type Boolean) (HitLocation :type Vector :default "0, 0, 0") (HitNormal :type Vector :default "0, 0, 0") (NormalImpulse :type Vector :default "0, 0, 0") (Hit :type Hit%20Result%20Structure%20%28by%20ref%29))
  (bind _returnvalue (Game|SpawnActorfromClass "/Game/BluenPrint/BP_OilSpill.BP_OilSpill_C" (Math|Transform|MakeTransform HitLocation (Math|Rotator|MakeRotfromZ HitNormal) "1.000000,1.000000,1.000000") "Undefined" "MultiplyWithRoot" 0 0))
  (if (Variables|Default|GetIsOnFire)
    (Default|SetonFire _returnvalue))
  (Actor|DestroyActor))

(fn ConstructionScript)