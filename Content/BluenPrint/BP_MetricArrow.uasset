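; BP_MetricArrow is a measuring marker that displays the distance between its actor origin and its Sphere component.
; The construction script writes that distance, rounded to a whole number of Unreal units, into a TextRender label.
; It also nudges the label along negative local X, Y and Z in proportion to the distance.
; The event graph holds only disabled placeholder events, so it adds no runtime logic.
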(event EventBeginPlay)

(event Collision|EventActorBeginOverlap
  (params (OtherActor :type Actor%20Object%20Reference)))

(event EventTick
  (params (DeltaSeconds :type Float%20%28single-precision%29)))

(fn ConstructionScript
  (bind _returnvalue (Transformation|GetActorLocation))
  (bind _sphere (Variables|Default|GetSphere))
  (bind _returnvalue_2 (Transformation|GetWorldLocation _sphere))
  (bind _returnvalue_3 (- _returnvalue _returnvalue_2))
  (bind _returnvalue_4 (Math|Vector|VectorLength _returnvalue_3))
  (bind _returnvalue_5 (Class|KismetMathLibrary|Round64 _returnvalue_4))
  (bind _returnvalue_6 (Math|Conversions|ToFloat(Integer) _returnvalue_5))
  (bind _returnvalue_7 (/ _returnvalue_6 -5e+01))
  (Rendering|Components|TextRender|SetText (Variables|Default|GetTextRender) (Utilities|Text|ToText(String) _returnvalue_5))
  (Transformation|AddLocalOffset (Variables|Default|GetTextRender) (Math|Vector|MakeVector _returnvalue_7 _returnvalue_7 _returnvalue_7) false false))