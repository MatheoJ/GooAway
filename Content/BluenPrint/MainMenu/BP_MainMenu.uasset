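; Main menu actor that presents three slime pawns as selectable options, each with a text label, beneath a large title.
; BeginPlay spawns slimes and text, finds BP_MainMenuPawn and aims it at the middle option.
; IA_Move steps the clamped index once per press, while Tick lerps pawn and camera toward that slime and removes 1-player HUD widgets.
; Shoot and Suck inputs are empty, and quit and level-loading logic is unconnected.
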(event Input|EnhancedActionEvents|EnhancedInputActionIA_Move
  (params (ActionValue :type Vector%202D%20Structure) (ElapsedSeconds :type Float%20%28double-precision%29) (TriggeredSeconds :type Float%20%28double-precision%29) (InputAction :type Input%20Action%20Object%20Reference :default "/Game/ThirdPerson/Input/Actions/IA_Move.IA_Move"))
  (:Triggered
    (if (not (Variables|Default|Getrotating))
      (Variables|Default|Setrotating true)
      (if (> (.x ActionValue) 0.0)
        (if (< (+ (Variables|Default|GetCurrentIndex) 1) 3)
          (bind _output_get (Variables|Default|SetCurrentIndex (+ (Variables|Default|GetCurrentIndex) 1))))
        (elif (> (+ (Variables|Default|GetCurrentIndex) -1) -1)
          (bind _output_get_2 (Variables|Default|SetCurrentIndex (+ (Variables|Default|GetCurrentIndex) -1)))))))
  (:Completed
    (Variables|Default|Setrotating false)
    (Development|PrintString "Hello")))

(event Input|EnhancedActionEvents|EnhancedInputActionIA_Suck
  (params (ActionValue :type Boolean) (ElapsedSeconds :type Float%20%28double-precision%29) (TriggeredSeconds :type Float%20%28double-precision%29) (InputAction :type Input%20Action%20Object%20Reference :default "/Game/ThirdPerson/Input/Actions/IA_Suck.IA_Suck")))

(event Input|EnhancedActionEvents|EnhancedInputActionIA_Shoot
  (params (ActionValue :type Boolean) (ElapsedSeconds :type Float%20%28double-precision%29) (TriggeredSeconds :type Float%20%28double-precision%29) (InputAction :type Input%20Action%20Object%20Reference :default "/Game/ThirdPerson/Input/Actions/IA_Shoot.IA_Shoot")))

(event EventBeginPlay
  (bind _returnvalue (Transformation|GetActorTransform))
  (bind _returnvalue_2 (Transformation|GetActorTransform))
  (bind _returnvalue_3 (Transformation|GetActorTransform))
  (bind _returnvalue_4 (Transformation|GetActorTransform))
  (bind _returnvalue_5 (Transformation|GetActorTransform))
  (bind _returnvalue_6 (+ (.location _returnvalue_3) "-400.000000,0.000000,0.000000"))
  (bind _returnvalue_7 (+ (.location _returnvalue_4) "400.000000,0.000000,0.000000"))
  (Utilities|FlowControl|Sequence
    (:then_0
      (Input|EnableInput (Game|GetPlayerController 0)))
    (:then_1
      (bind _returnvalue_8 (Game|SpawnActorfromClass "/Game/BluenPrint/Slime/BP_ElectricSlimePawn.BP_ElectricSlimePawn_C" (Math|Transform|MakeTransform _returnvalue_7 "0.000000,-90.000000,0.000000" (.scale _returnvalue_4)) "Undefined" "MultiplyWithRoot" 0 0))
      (Utilities|Array|Add (Variables|Default|GetSlimeOptions) _returnvalue_8)
      (bind _returnvalue_9 (Game|SpawnActorfromClass "/Script/Engine.TextRenderActor" (Math|Transform|MakeTransform (+ _returnvalue_7 "0.000000,-10.000000,50.000000") "0.000000,-90.000000,0.000000" (* (.scale _returnvalue_4) 2)) "Undefined" "MultiplyWithRoot" 0 0))
      (Utilities|Array|Add (Variables|Default|GetTextOptions) _returnvalue_9)
      (bind _returnvalue_10 (Game|SpawnActorfromClass "/Game/BluenPrint/Slime/BP_WaterSlimePawn.BP_WaterSlimePawn_C" (Math|Transform|MakeTransform (.location _returnvalue_5) "0.000000,-90.000000,0.000000" (.scale _returnvalue_5)) "Undefined" "MultiplyWithRoot" 0 0))
      (Utilities|Array|Add (Variables|Default|GetSlimeOptions) _returnvalue_10)
      (bind _returnvalue_11 (Game|SpawnActorfromClass "/Script/Engine.TextRenderActor" (Math|Transform|MakeTransform (+ (.location _returnvalue) "0.000000,-10.000000,50.000000") "0.000000,-90.000000,0.000000" (* (.scale _returnvalue) 2)) "Undefined" "MultiplyWithRoot" 0 0))
      (Utilities|Array|Add (Variables|Default|GetTextOptions) _returnvalue_11)
      (bind _returnvalue_12 (Game|SpawnActorfromClass "/Game/BluenPrint/Slime/BP_OilSlimePawn.BP_OilSlimePawn_C" (Math|Transform|MakeTransform _returnvalue_6 "0.000000,-90.000000,0.000000" (.scale _returnvalue_3)) "Undefined" "MultiplyWithRoot" 0 0))
      (Utilities|Array|Add (Variables|Default|GetSlimeOptions) _returnvalue_12)
      (bind _returnvalue_13 (Game|SpawnActorfromClass "/Script/Engine.TextRenderActor" (Math|Transform|MakeTransform (+ _returnvalue_6 "0.000000,-10.000000,50.000000") "0.000000,-90.000000,0.000000" (* (.scale _returnvalue_3) 2)) "Undefined" "MultiplyWithRoot" 0 0))
      (Utilities|Array|Add (Variables|Default|GetTextOptions) _returnvalue_13)
      (for (_array_element _array_index) (Variables|Default|GetTextOptions)
        (Rendering|Components|TextRender|SetText (Variables|/Script/Engine.TextRenderActor|GetTextRender _array_element) (Utilities|Array|Get(acopy) (Variables|Default|GetMenuOptions) _array_index))
        (Rendering|Components|TextRender|SetHorizontalAlignment (Variables|/Script/Engine.TextRenderActor|GetTextRender _array_element) "EHTA_Center")
        (Class|TextRenderComponent|SetVerticalAlignment (Variables|/Script/Engine.TextRenderActor|GetTextRender _array_element) "EVRTA_TextCenter")))
    (:then_2
      (bind _returnvalue_14 (Actor|GetActorOfClass "/Game/BluenPrint/MainMenu/BP_MainMenuPawn.BP_MainMenuPawn_C"))
      (Variables|Default|SetPawn _returnvalue_14))
    (:then_3
      (bind _output_get (Variables|Default|SetCurrentIndex 1))
      (CallFunction|LookatIndex _output_get))
    (:then_4
      (bind _returnvalue_15 (Game|SpawnActorfromClass "/Script/Engine.TextRenderActor" (Math|Transform|MakeTransform (+ (.location _returnvalue_2) "0.000000,0.000000,200.000000") "0.000000,-90.000000,0.000000" (* (.scale _returnvalue_2) 5)) "Undefined" "MultiplyWithRoot" 0 0))
      (Rendering|Components|TextRender|SetText (Variables|/Script/Engine.TextRenderActor|GetTextRender _returnvalue_15) (Variables|Default|GetValue))
      (Rendering|Components|TextRender|SetHorizontalAlignment (Variables|/Script/Engine.TextRenderActor|GetTextRender _returnvalue_15) "EHTA_Center")
      (Class|TextRenderComponent|SetVerticalAlignment (Variables|/Script/Engine.TextRenderActor|GetTextRender _returnvalue_15) "EVRTA_TextCenter"))
    (:then_5
      (Actor|GetAllActorsOfClass 0))))

(event Collision|EventActorBeginOverlap
  (params (OtherActor :type Actor%20Object%20Reference)))

(event EventTick
  (params (DeltaSeconds :type Float%20%28single-precision%29))
  (bind _pawn (Variables|Default|GetPawn))
  (bind _slimeoptions (Variables|Default|GetSlimeOptions))
  (bind _currentindex (Variables|Default|GetCurrentIndex))
  (bind _output (Utilities|Array|Get(acopy) _slimeoptions _currentindex))
  (bind _camera (Variables|/Game/BluenPrint/MainMenu/BP_MainMenuPawn.BP_MainMenuPawn_C|GetCamera _pawn))
  (bind _returnvalue (Transformation|GetActorLocation _output))
  (Transformation|SetActorRotation _pawn (Math|Rotator|Lerp(Rotator) (Transformation|GetActorRotation _pawn) (Math|Rotator|FindLookatRotation (Transformation|GetActorLocation _pawn) _returnvalue) 0.02))
  (Transformation|SetWorldRotation _camera (Math|Rotator|Lerp(Rotator) (Transformation|GetWorldRotation _camera) (Math|Rotator|FindLookatRotation (Transformation|GetWorldLocation _camera) _returnvalue) 0.02) false false)
  (bind _foundwidgets (Widget|GetAllWidgetsOfClass "/Game/Widgets/New_HUD/WB_HUD_1player.WB_HUD_1player_C" true))
  (for _array_element _foundwidgets
    (Widget|RemovefromParent _array_element)))

(fn ConstructionScript)

(fn LookatIndex
  (params (Dimension%201 :type Integer))
  (bind _pawn (Variables|Default|GetPawn))
  (bind _slimeoptions (Variables|Default|GetSlimeOptions))
  (bind _output (Utilities|Array|Get(acopy) _slimeoptions Dimension%201))
  (bind _camera (Variables|/Game/BluenPrint/MainMenu/BP_MainMenuPawn.BP_MainMenuPawn_C|GetCamera _pawn))
  (bind _returnvalue (Transformation|GetActorLocation _output))
  (Transformation|SetActorRotation _pawn (Math|Rotator|FindLookatRotation (Transformation|GetActorLocation _pawn) _returnvalue))
  (Transformation|SetWorldRotation _camera (Math|Rotator|FindLookatRotation (Transformation|GetWorldLocation _camera) _returnvalue) false false))