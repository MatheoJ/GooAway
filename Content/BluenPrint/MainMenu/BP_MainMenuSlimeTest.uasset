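; Main menu controller that presents Exit, Play and Credits as three spawned slime pawns: electric, water and oil.
; Move input steps the selection and highlights its label mesh, while Tick turns the player character and camera toward that slime.
; Once the character is loaded and the slime stops moving to the cannon, Tick quits, opens MainLevel, or shows credits and respawns the oil slime.
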(event Input|EnhancedActionEvents|EnhancedInputActionIA_Move
  (params (ActionValue :type Vector%202D%20Structure) (ElapsedSeconds :type Float%20%28double-precision%29) (TriggeredSeconds :type Float%20%28double-precision%29) (InputAction :type Input%20Action%20Object%20Reference :default "/Game/ThirdPerson/Input/Actions/IA_Move.IA_Move"))
  (bind _exit (Variables|Default|GetExit))
  (bind _credits (Variables|Default|GetCredits))
  (bind _play (Variables|Default|GetPlay))
  (bind _staticmeshcomponent (Variables|/Script/Engine.StaticMeshActor|GetStaticMeshComponent _credits))
  (bind _staticmeshcomponent_2 (Variables|/Script/Engine.StaticMeshActor|GetStaticMeshComponent _exit))
  (bind _staticmeshcomponent_3 (Variables|/Script/Engine.StaticMeshActor|GetStaticMeshComponent _play))
  (:Triggered
    (if (not (Variables|Default|Getrotating))
      (Variables|Default|Setrotating true)
      (if (> (.x ActionValue) 0.0)
        (if (< (+ (Variables|Default|GetCurrentIndex) 1) 3)
          (Variables|Default|SetCurrentIndex (+ (Variables|Default|GetCurrentIndex) 1))
          (switch int (Variables|Default|GetCurrentIndex) :!label _label
            (:0
              (Rendering|Material|SetColorParameterValueonMaterials _staticmeshcomponent_2 "Color" "(R=0.000000,G=0.400000,B=1.000000,A=1.000000)")
              (Rendering|Material|SetColorParameterValueonMaterials _staticmeshcomponent "Color" "(R=1.000000,G=1.000000,B=1.000000,A=1.000000)")
              (Rendering|Material|SetColorParameterValueonMaterials _staticmeshcomponent_3 "Color" "(R=1.000000,G=1.000000,B=1.000000,A=1.000000)"))
            (:1
              (Rendering|Material|SetColorParameterValueonMaterials _staticmeshcomponent_3 "Color" "(R=0.000000,G=0.400000,B=1.000000,A=1.000000)")
              (Rendering|Material|SetColorParameterValueonMaterials _staticmeshcomponent "Color" "(R=1.000000,G=1.000000,B=1.000000,A=1.000000)")
              (Rendering|Material|SetColorParameterValueonMaterials _staticmeshcomponent_2 "Color" "(R=1.000000,G=1.000000,B=1.000000,A=1.000000)"))
            (:2
              (Rendering|Material|SetColorParameterValueonMaterials _staticmeshcomponent "Color" "(R=0.000000,G=0.400000,B=1.000000,A=1.000000)")
              (Rendering|Material|SetColorParameterValueonMaterials _staticmeshcomponent_3 "Color" "(R=1.000000,G=1.000000,B=1.000000,A=1.000000)")
              (Rendering|Material|SetColorParameterValueonMaterials _staticmeshcomponent_2 "Color" "(R=1.000000,G=1.000000,B=1.000000,A=1.000000)"))))
        (elif (> (+ (Variables|Default|GetCurrentIndex) -1) -1)
          (Variables|Default|SetCurrentIndex (+ (Variables|Default|GetCurrentIndex) -1))
          (goto _label)))))
  (:Completed
    (Variables|Default|Setrotating false)))

(event Input|EnhancedActionEvents|EnhancedInputActionIA_Suck
  (params (ActionValue :type Boolean) (ElapsedSeconds :type Float%20%28double-precision%29) (TriggeredSeconds :type Float%20%28double-precision%29) (InputAction :type Input%20Action%20Object%20Reference :default "/Game/ThirdPerson/Input/Actions/IA_Suck.IA_Suck")))

(event Input|EnhancedActionEvents|EnhancedInputActionIA_Shoot
  (params (ActionValue :type Boolean) (ElapsedSeconds :type Float%20%28double-precision%29) (TriggeredSeconds :type Float%20%28double-precision%29) (InputAction :type Input%20Action%20Object%20Reference :default "/Game/ThirdPerson/Input/Actions/IA_Shoot.IA_Shoot")))

(event EventBeginPlay
  (bind _returnvalue (Transformation|GetActorTransform))
  (bind _returnvalue_2 (Transformation|GetActorTransform))
  (bind _returnvalue_3 (Transformation|GetActorTransform))
  (Utilities|FlowControl|Sequence
    (:then_0
      (Input|EnableInput (Game|GetPlayerController 0)))
    (:then_1
      (bind _returnvalue_4 (Game|SpawnActorfromClass "/Game/BluenPrint/Slime/BP_ElectricSlimePawn.BP_ElectricSlimePawn_C" (Math|Transform|MakeTransform (+ (.location _returnvalue) "0.000000,-400.000000,0.000000") (Math|Rotator|MakeRotator 0.0 -45.0 -212.3502) (.scale _returnvalue)) "Undefined" "MultiplyWithRoot" 0 false 0))
      (Class|Pawn|DetachfromControllerPendingDestroy _returnvalue_4)
      (Utilities|Array|Add (Variables|Default|GetSlimeOptions) _returnvalue_4)
      (bind _returnvalue_5 (Game|SpawnActorfromClass "/Game/BluenPrint/Slime/BP_WaterSlimePawn.BP_WaterSlimePawn_C" (Math|Transform|MakeTransform (.location _returnvalue_2) (Math|Rotator|MakeRotator 0.0 -45.0 -1.8e+02) (.scale _returnvalue_2)) "Undefined" "MultiplyWithRoot" 0 false 0))
      (Class|Pawn|DetachfromControllerPendingDestroy _returnvalue_5)
      (Utilities|Array|Add (Variables|Default|GetSlimeOptions) _returnvalue_5)
      (bind _returnvalue_6 (Game|SpawnActorfromClass "/Game/BluenPrint/Slime/BP_OilSlimePawn.BP_OilSlimePawn_C" (Math|Transform|MakeTransform (+ (.location _returnvalue_3) "0.000000,400.000000,0.000000") (Math|Rotator|MakeRotator 0.0 -45.0 -1.5e+02) (.scale _returnvalue_3)) "Undefined" "MultiplyWithRoot" 0 false 0))
      (Class|Pawn|DetachfromControllerPendingDestroy _returnvalue_6)
      (Utilities|Array|Add (Variables|Default|GetSlimeOptions) _returnvalue_6))
    (:then_2
      (Variables|Default|SetCurrentIndex 1))
    (:then_4
      (Rendering|Material|SetColorParameterValueonMaterials (Variables|/Script/Engine.StaticMeshActor|GetStaticMeshComponent (Variables|Default|GetPlay)) "Color" "(R=0.000000,G=0.400142,B=1.000000,A=1.000000)"))
    (:then_5
      (Utilities|FlowControl|DelayUntilNextTick)
      (bind _returnvalue_7 (Actor|GetActorOfClass "/Game/ThirdPerson/Blueprints/BP_ThirdPersonCharacter_onlyBP.BP_ThirdPersonCharacter_onlyBP_C"))
      (bind _outactors (Actor|GetAllActorsOfClass "/Game/ThirdPerson/Blueprints/BP_ThirdPersonCharacter_onlyBP.BP_ThirdPersonCharacter_onlyBP_C"))
      (for _array_element _outactors
        (if (!= _returnvalue_7 _array_element)
          (bind _output_get (Variables|Default|SetTrueCharacter _array_element))
          (Variables|Default|SetinitDone true))))))

(event EventTick
  (params (DeltaSeconds :type Float%20%28single-precision%29))
  (bind _returnvalue (Transformation|GetActorTransform))
  (bind _truecharacter (Variables|Default|GetTrueCharacter))
  (bind _slimeoptions (Variables|Default|GetSlimeOptions))
  (bind _currentindex (Variables|Default|GetCurrentIndex))
  (bind _truecharacter_2 (Variables|Default|GetTrueCharacter))
  (bind _output (Utilities|Array|Get(acopy) _slimeoptions _currentindex))
  (bind _followcamera (Variables|/Game/ThirdPerson/Blueprints/BP_ThirdPersonCharacter_onlyBP.BP_ThirdPersonCharacter_onlyBP_C|GetFollowCamera _truecharacter))
  (bind _mesh (Variables|/Script/Engine.Character|GetMesh _truecharacter))
  (bind _returnvalue_2 (Transformation|GetActorLocation _output))
  (if (Variables|Default|GetinitDone)
    (Variables|Default|SetDelta%20Seconds DeltaSeconds)
    (if (and (Variables|/Game/ThirdPerson/Blueprints/BP_ThirdPersonCharacter_onlyBP.BP_ThirdPersonCharacter_onlyBP_C|GetLoaded _truecharacter_2) (not (Variables|/Game/ThirdPerson/Blueprints/BP_ThirdPersonCharacter_onlyBP.BP_ThirdPersonCharacter_onlyBP_C|GetSlimeMovingToCanon _truecharacter_2)))
      (switch int (Variables|Default|GetCurrentIndex)
        (:Default
          (Game|QuitGame 0 "Quit" false :!label _label))
        (:0
          (goto _label))
        (:1
          (Game|OpenLevel(byObjectReference) "/Game/Gyms/GameLevels/MainLevel.MainLevel"))
        (:2
          (Utilities|FlowControl|DoOnce false :!label _label_2
            (:Completed
              (bind _returnvalue_3 (UserInterface|CreateWidget "/Game/Widgets/WBCredits.WBCredits_C" (Game|GetPlayerController 0)))
              (UserInterface|Viewport|AddtoViewport _returnvalue_3 0)
              (Utilities|Array|RemoveIndex (Variables|Default|GetSlimeOptions) 2)
              (bind _returnvalue_4 (Game|SpawnActorfromClass "/Game/BluenPrint/Slime/BP_OilSlimePawn.BP_OilSlimePawn_C" (Math|Transform|MakeTransform (+ (.location _returnvalue) "0.000000,400.000000,0.000000") (Math|Rotator|MakeRotator 0.0 -45.0 -1.5e+02) (.scale _returnvalue)) "Undefined" "MultiplyWithRoot" 0 false 0))
              (Class|Pawn|DetachfromControllerPendingDestroy _returnvalue_4)
              (Utilities|Array|Add (Variables|Default|GetSlimeOptions) _returnvalue_4)
              (Variables|/Game/ThirdPerson/Blueprints/BP_ThirdPersonCharacter_onlyBP.BP_ThirdPersonCharacter_onlyBP_C|SetLoaded (Variables|Default|GetTrueCharacter) false)
              (goto _label_2 Reset)))))
      (else
        (Transformation|SetWorldRotation _mesh (Math|Rotator|Lerp(Rotator) (Transformation|GetWorldRotation _mesh) (Math|Rotator|CombineRotators "0.000000,270.000000,0.000000" (Math|Rotator|FindLookatRotation (Transformation|GetActorLocation _truecharacter) _returnvalue_2)) (* (Variables|Default|GetDelta%20Seconds) 7.0)) false false)
        (Transformation|SetWorldRotation _followcamera (Math|Rotator|Lerp(Rotator) (Transformation|GetWorldRotation _followcamera) (Math|Rotator|FindLookatRotation (Transformation|GetWorldLocation _followcamera) _returnvalue_2) (* (Variables|Default|GetDelta%20Seconds) 7.0)) false false)
        (Utilities|FlowControl|DoOnce false
          (:Completed
            (bind _foundwidgets (Widget|GetAllWidgetsOfClass "/Game/Widgets/New_HUD/WB_HUD_1player.WB_HUD_1player_C" true))
            (for _array_element _foundwidgets
              (Variables|/Script/UMG.Widget|SetVisibility (Variables|/Game/Widgets/New_HUD/WB_HUD_1player.WB_HUD_1player_C|GetWB_Cross _array_element) "Hidden"))))))))

(fn ConstructionScript)