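; BP_SlimeNavigation is a key-driven front end for building, loading and debugging a custom slime navigation grid.
; On BeginPlay it caches the first SlimeNavGridBuilder actor found and prints a key hint.
; R has the builder rebuild the grid and then reloads it, H reloads and logs the node count, and Q draws node connections.
; The hint also advertises K for rebuilding, but no K binding exists in this graph.
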(event EventBeginPlay
  (Utilities|FlowControl|Sequence
    (:then_0
      (bind _outactors (Actor|GetAllActorsOfClass "/Script/Pompastronautes.SlimeNavGridBuilder"))
      (if (> (Utilities|Array|Length _outactors) 0)
        (Variables|Default|SetSlimeNavGridBuilder (Utilities|Array|Get(acopy) _outactors))
        (Development|PrintString "Slime Navigation: R or K - rebuild, Q - show connections" true true "(R=0.000000,G=0.660000,B=1.000000,A=1.000000)" 2e+01)))))

(event Input|KeyboardEvents|R
  (params (Key :type Key%20Structure :default "None"))
  (:Pressed
    (Development|PrintString "Building Grid...")
    (Class|SlimeNavGridBuilder|BuildGrid (Variables|Default|GetSlimeNavGridBuilder))
    (Development|PrintString "Custom Nav Grid has been built")
    (Class|SlimeNavigation|LoadGrid)))

(event Input|KeyboardEvents|Q
  (params (Key :type Key%20Structure :default "None"))
  (:Pressed
    (Class|SlimeNavigation|DrawDebugRelations)))

(event Input|KeyboardEvents|H
  (params (Key :type Key%20Structure :default "None"))
  (:Pressed
    (bind _returnvalue (Class|SlimeNavigation|LoadGrid))
    (bind _returnvalue_2 (Class|SlimeNavigation|GetNavNodesCount))
    (Development|PrintString (Utilities|String|Append "Custom Nav Grid Load Result: " (Utilities|String|ToString(Boolean) _returnvalue) " Loaded: " (Utilities|String|ToString(Integer) _returnvalue_2)) false)))

(fn ConstructionScript)