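; AI controller for an oil slime enemy that fires a BP_OilAttack actor at the player.
; Tick counts TimeSinceLastAttack down as a cooldown, clamped between zero and the attack interval.
; When that timer is nearly expired, AttackPlayer spawns the attack at the controlled pawn, rotated toward a point above the player.
; AttackPlayer does not reset the timer, and nothing in these graphs calls it.
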(event EventBeginPlay
  (|CallParentFunction) ; This node is disabled and will not be called.\nDrag off pins to build functionality.
)

(event EventTick
  (params (DeltaSeconds :type Float%20%28single-precision%29))
  (Variables|Default|SetTimeSinceLastAttack (Math|Float|Clamp(Float) (- (Variables|Default|GetTimeSinceLastAttack) DeltaSeconds) 0.0 (Variables|Default|GetTimeBeeweenAttack)))
  (|CallParentFunction DeltaSeconds))

(fn ConstructionScript
  (|CallParentFunction))

(fn AttackPlayer
  (params (Player :type Actor%20Object%20Reference))
  (bind _returnvalue (Pawn|GetControlledPawn))
  (bind _returnvalue_2 (Transformation|GetActorLocation _returnvalue))
  (if (not (> (Variables|Default|GetTimeSinceLastAttack) 0.1))
    (Game|SpawnActorfromClass "/Game/BluenPrint/BP_OilAttack.BP_OilAttack_C" (Math|Transform|MakeTransform _returnvalue_2 (Math|Rotator|MakeRotfromX (- (+ (Transformation|GetActorLocation Player) "0.000000,0.000000,120.000000") _returnvalue_2)) "1.000000,1.000000,1.000000") "AdjustIfPossibleButAlwaysSpawn" "MultiplyWithRoot" 0 0)))