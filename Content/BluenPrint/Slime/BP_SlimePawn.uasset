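; BP_SlimePawn is a slime pawn that gives each instance its own color and randomized animated look.
; BeginPlay applies a dynamic material to the Sphere with the Color variable and random pulse, band and noise parameters.
; Tick feeds the sphere's negated forward vector into the material's SlimeDirection parameter.
; The Collision overlap event is empty; logic to nudge overlapping slimes horizontally exists but is disconnected.
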(event OnComponentBeginOverlap(Collision)
  (params (OverlappedComponent :type Primitive%20Component%20Object%20Reference) (OtherActor :type Actor%20Object%20Reference) (OtherComp :type Primitive%20Component%20Object%20Reference) (OtherBodyIndex :type Integer) (bFromSweep :type Boolean) (SweepResult :type Hit%20Result%20Structure%20%28by%20ref%29)))

(event EventBeginPlay
  (bind _returnvalue (Rendering|Material|CreateDynamicMaterialInstance (Variables|Default|GetMaterialParent) "MI_Slimemat" "None" :!class /Script/Engine.KismetMaterialLibrary))
  (Rendering|Material|SetVectorParameterValue _returnvalue "BaseColor" (Variables|Default|GetColor) :!class /Script/Engine.MaterialInstanceDynamic)
  (Rendering|Material|SetMaterial (Variables|Default|GetSphere) 0 _returnvalue)
  (Rendering|Material|SetScalarParameterValueonMaterials (Variables|Default|GetSphere) "PulseIntensity" (Math|Random|RandomFloatinRange 1.0 4.0))
  (Rendering|Material|SetScalarParameterValueonMaterials (Variables|Default|GetSphere) "PulseSpeed" (Math|Random|RandomFloatinRange 1.0 2.0))
  (Rendering|Material|SetVectorParameterValueonMaterials (Variables|Default|GetSphere) "NoiseWidth" (Math|Vector|MakeVector (Math|Random|RandomFloatinRange 0.0 1.0) (Math|Random|RandomFloatinRange 0.0 1.0) (Math|Random|RandomFloatinRange 0.0 1.0)))
  (Rendering|Material|SetScalarParameterValueonMaterials (Variables|Default|GetSphere) "BandIntensity" (Math|Random|RandomFloatinRange 1.0 2.0))
  (Rendering|Material|SetScalarParameterValueonMaterials (Variables|Default|GetSphere) "BandSpeed" (Math|Random|RandomFloatinRange 1.0 2.0)))

(event EventTick
  (params (DeltaSeconds :type Float%20%28single-precision%29))
  (bind _sphere (Variables|Default|GetSphere))
  (Rendering|Material|SetVectorParameterValueonMaterials _sphere "SlimeDirection" (* (Math|Vector|GetForwardVector (Transformation|GetWorldRotation _sphere)) (Math|Conversions|ToVector(Float) -1.0))))

(fn ConstructionScript)