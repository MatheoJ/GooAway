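; AI controller for slime pawns that crawl toward an objective and leap at players.
; BeginPlay gets the nearest objective's attack point from the objective manager, seeds the blackboard and runs the behavior tree.
; Move follows custom SlimeNavigation paths, using node normals to offset and orient the pawn along surfaces.
; Jumps are physics impulses ended by sphere trace; hitting a Character attaches the slime and halts its tick and brain logic.
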(event Custom|OnFindPathTick
  (if (Variables|Default|GetMustMove)
    (CallFunction|UpdateLocalMoveDestination)
    (if (not (Variables|Default|GetLocalPathFound))
      (Variables|Default|SetMustMove false))))

(event EventBeginPlay
  (bind _objectiflocation (Variables|Default|GetObjectifLocation))
  (Utilities|FlowControl|Sequence
    (:then_0
      (bind _outactors (Actor|GetAllActorsOfClass "/Script/Pompastronautes.SlimeNavigation"))
      (if (> (Utilities|Array|Length _outactors) 0)
        (Variables|Default|SetNavigation (Utilities|Array|Get(acopy) _outactors))
        (Utilities|Time|SetTimerbyEvent (delegate Custom|OnFindPathTick) (Variables|Default|GetUpdateLocalDestinationInterval) true)
        (else
          (Development|PrintString "No navigation actor for movement" true true "(R=1.000000,G=0.000000,B=0.142920,A=1.000000)"))))
    (:then_1
      (CallFunction|UpdateObjectifLocation))
    (:then_2
      ;[1 1 1] BT and BB SetUP
      (bind _blackboardcomponent (Class|AIController|UseBlackboard "/Game/BluenPrint/Slime/Behavior/SlimeBB.SlimeBB"))
      (AI|Components|Blackboard|SetValueasVector _blackboardcomponent (Variables|Default|GetObjectiveLocation) _objectiflocation)
      (AI|Components|Blackboard|SetValueasBool _blackboardcomponent (Variables|Default|GetHasObjective) (Utilities|Operators|NotEqual(!=) :A _objectiflocation :ErrorTolerance 0.001))
      (AI|RunBehaviorTree (Variables|Default|GetBehaviourTree)))
    (:then_3
      (Variables|Default|SetControlledPawn (Pawn|GetControlledPawn))
      (bind _outactors_2 (Actor|GetAllActorsOfClass "/Game/ThirdPerson/Blueprints/BP_ThirdPersonCharacter_onlyBP.BP_ThirdPersonCharacter_onlyBP_C"))
      (Variables|Default|SetPlayers _outactors_2))))

(event EventTick
  (params (DeltaSeconds :type Float%20%28single-precision%29))
  (bind _returnvalue (Pawn|GetControlledPawn))
  (Utilities|FlowControl|Sequence
    (:then_1
      (if (Variables|Default|GetIsSlimeJumping)
        ;[0.15 0.15 0.15 0.5] Handling Jump
        (if (Variables|Default|GetCanStopJump)
          (bind _output_get (Variables|Default|SetControlledPawn (Pawn|GetControlledPawn)))
          (bind (_outhit _returnvalue_2) (Collision|SphereTraceByChannel (Transformation|GetActorLocation _output_get) (Transformation|GetActorLocation _output_get) (- (Variables|Default|GetHeightOfPawnFromGround) 3.0) "TraceTypeQuery5" false 0 "None"))
          (if _returnvalue_2
            (Class|KismetSystemLibrary|IsObjectOfSoftClass (.hitactor _outhit) "/Script/Engine.Character"
              (:True
                (Class|BPIInterface|SlimeJump(Message) (Variables|Default|GetControlledPawn) true (Variables|Default|GetIsSlimeJumping))
                (Transformation|AttachActorToActor (Variables|Default|GetControlledPawn) (.hitactor _outhit) "None" "KeepWorld" "KeepRelative" "KeepWorld" true)
                (Actor|Tick|SetActorTickEnabled false)
                (AI|Logic|StopLogic (Variables|Default|GetBrainComponent) "We Are Stuck To the player we Need To Wait till is launch of the player"))
              (:False
                (Class|BPIInterface|SlimeJump(Message) (Variables|Default|GetControlledPawn) false (Variables|Default|GetIsSlimeJumping))
                (Development|PrintString (Utilities|GetDisplayName (.hitactor _outhit)))))
            (Variables|Default|SetIsSlimeJumping false)
            (Variables|Default|SetMoveDestination "0, 0, 0")
            (bind _asbp_slime_pawn (Utilities|Casting|CastToBP_SlimePawn (Variables|Default|GetControlledPawn)))
            (Physics|SetSimulatePhysics (Variables|/Game/BluenPrint/Slime/BP_SlimePawn.BP_SlimePawn_C|GetCollision _asbp_slime_pawn) false)
            (Collision|SetCollisionEnabled (Variables|/Game/BluenPrint/Slime/BP_SlimePawn.BP_SlimePawn_C|GetCollision _asbp_slime_pawn) "QueryOnly")
            (Default|CallJumpComplete true)))
        (else
          (Utilities|FlowControl|Sequence
            (:then_0
              ;[1 1 1] Check finish
              (if (< (Math|Vector|VectorLength (- (Transformation|GetActorLocation (Pawn|GetControlledPawn)) (Variables|Default|GetMoveDestination))) (* (Variables|Default|GetMoveSpeed) 0.2))
                (Variables|Default|SetMustMove false)
                (Default|CallMovementComplete true)))
            (:then_1
              ;[1 1 1] Rotation
              (if (Variables|Default|GetMustRotate)
                (if (Utilities|Enum|NotEqual(Enum) (Transformation|GetActorRotation (Pawn|GetControlledPawn)) (Variables|Default|GetRotationDestination) 0.01)
                  (Transformation|SetActorRotation (Pawn|GetControlledPawn) (Math|Interpolation|RInterpTo (Transformation|GetActorRotation (Pawn|GetControlledPawn)) (Variables|Default|GetRotationDestination) DeltaSeconds (Variables|Default|GetRotationSpeed)))
                  (else
                    (Variables|Default|SetMustRotate false)))))
            (:then_2
              ;[1 1 1] Move
              (if (Math|Boolean|ANDBoolean true (Variables|Default|GetMustMove) (Variables|Default|GetMustMoveLocal))
                (Variables|Default|SetNormalToDestinationBeforeMove (Utilities|GetNormaltoLocalDestination))
                (Pawn|Input|AddMovementInput _returnvalue (Transformation|GetActorForwardVector _returnvalue) (Variables|Default|GetMoveSpeed) false)
                (if (or (Math|Vector|NotEqual(Vector) (Utilities|GetNormaltoLocalDestination) (Variables|Default|GetNormalToDestinationBeforeMove) 0.1) (< (Math|Vector|VectorLength (- (Transformation|GetActorLocation (Pawn|GetControlledPawn)) (Variables|Default|GetLocalMoveDestination))) (* (Variables|Default|GetHeightOfPawnFromGround) 1.6)))
                  (Utilities|Array|RemoveIndex (Variables|Default|GetCurrentPath))
                  (CallFunction|UpdateLocalMoveDestination))))))))))

(event EventLaunchSlimeinDirection
  (params (Direction :type Vector :default "0, 0, 0"))
  (Variables|Default|SetIsSlimeJumping true)
  (bind _asbp_slime_pawn (Utilities|Casting|CastToBP_SlimePawn (Pawn|GetControlledPawn)))
  (Variables|/Game/BluenPrint/Slime/BP_SlimePawn.BP_SlimePawn_C|SetbIsJumping _asbp_slime_pawn true)
  (Collision|SetCollisionEnabled (Variables|/Game/BluenPrint/Slime/BP_SlimePawn.BP_SlimePawn_C|GetCollision _asbp_slime_pawn) "QueryAndPhysics")
  (Physics|SetSimulatePhysics (Variables|/Game/BluenPrint/Slime/BP_SlimePawn.BP_SlimePawn_C|GetCollision _asbp_slime_pawn) true)
  (Physics|AddImpulse (Variables|/Game/BluenPrint/Slime/BP_SlimePawn.BP_SlimePawn_C|GetCollision _asbp_slime_pawn) (* (Math|Vector|Normalize Direction 0.001) (Variables|Default|GetStartLaunchSpeed)) "None" true)
  (Variables|Default|SetCanStopJump false)
  (Utilities|Time|SetTimerbyFunctionName 0 "SetCanStopJump" 0.1))

(fn ConstructionScript)

(fn Move
  (params (Destination :type Vector) (PathJitter :type Float%20%28double-precision%29))
  (bind _returnvalue (Class|SlimeNavigation|FindClosestNodeLocation (Variables|Default|GetNavigation) Destination))
  (if (not (Math|Vector|Equal(Vector) _returnvalue (Variables|Default|GetMoveDestination) 0.0001))
    (bind _output_get (Variables|Default|SetMoveDestination _returnvalue))
    (bind _returnvalue_2 (Class|SlimeNavigation|FindPath (Variables|Default|GetNavigation) (Transformation|GetActorLocation (Pawn|GetControlledPawn)) _output_get PathJitter))
    (bind _output_get_2 (Variables|Default|SetCurrentPath _returnvalue_2))
    (Utilities|Array|RemoveIndex _output_get_2)
    (CallFunction|UpdateLocalMoveDestination)
    (if (Variables|Default|GetLocalPathFound)
      (Variables|Default|SetMustMove true))))

(fn UpdateLocalMoveDestination
  (bind _currentpath (Variables|Default|GetCurrentPath))
  (bind _output (Utilities|Array|Get(acopy) _currentpath))
  (if (> (Utilities|Array|Length (Variables|Default|GetCurrentPath)) 0)
    (bind _returnvalue (Class|SlimeNavigation|FindClosestNodeNormal (Variables|Default|GetNavigation) _output))
    (Variables|Default|SetLocalMoveDestination (+ _output (* _returnvalue (Variables|Default|GetHeightOfPawnFromGround))))
    (Variables|Default|SetMoveNormal _returnvalue)
    (Variables|Default|SetLocalPathFound true)
    (Variables|Default|SetMustMoveLocal true)
    (CallFunction|UpdateRotationParams)
    (else
      (Variables|Default|SetLocalPathFound false)
      (Variables|Default|SetMustMoveLocal false)))
  (if (Variables|Default|GetDEBUG_DrawPath)
    ;[1 1 1] Debug
    (Rendering|Debug|DrawDebugSphere (Variables|Default|GetLocalMoveDestination) 0.0 6 "(R=1.000000,G=0.000000,B=0.000000,A=1.000000)" (Variables|Default|GetUpdateLocalDestinationInterval))
    (for _array_element (Variables|Default|GetCurrentPath)
      (Rendering|Debug|DrawDebugSphere _array_element 6.0 12 "(R=0.000000,G=0.099035,B=1.000000,A=1.000000)" (Variables|Default|GetUpdateLocalDestinationInterval) 2.0))
    (bind _returnvalue_2 (Class|SlimeNavigation|FindClosestNodeLocation (Variables|Default|GetNavigation) (Variables|Default|GetMoveDestination)))
    (Rendering|Debug|DrawDebugSphere _returnvalue_2 7.0 12 "(R=0.124380,G=1.000000,B=0.158918,A=1.000000)" (Variables|Default|GetUpdateLocalDestinationInterval))))

(fn UpdateRotationParams
  (Variables|Default|SetRotationBeforeMove (Transformation|GetActorRotation (Pawn|GetControlledPawn)))
  (Variables|Default|SetRotationDestination (Math|Rotator|MakeRotfromXZ (- (Variables|Default|GetLocalMoveDestination) (Transformation|GetActorLocation (Pawn|GetControlledPawn))) (Variables|Default|GetMoveNormal)))
  (Variables|Default|SetMustRotate (Utilities|Enum|NotEqual(Enum) (Variables|Default|GetRotationDestination) (Variables|Default|GetRotationBeforeMove) 0.01)))

(fn LaunchtoPlayer
  (params (PlayerTarget :type Actor%20Object%20Reference))
  (CallFunction|LaunchinDirection (- (+ (Transformation|GetActorLocation PlayerTarget) (Math|Vector|MakeVector 0.0 0.0 (Math|Random|RandomFloatinRange 0.0 1.8e+02))) (Transformation|GetActorLocation (Pawn|GetControlledPawn)))))

(fn SetCanStopJump
  (Variables|Default|SetCanStopJump true))

(fn UpdateObjectifLocation
  (bind _outactors (Actor|GetAllActorsOfClass "/Game/BluenPrint/BP_SlimeObjectifManager.BP_SlimeObjectifManager_C"))
  (if (> (Utilities|Array|Length _outactors) 0)
    (bind _returnvalue (Class|SlimeObjectifManager|GetClossestObjectif (Utilities|Array|Get(acopy) _outactors) self))
    (bind _output_get (Variables|Default|SetCurrentObjectif _returnvalue))
    (bind _returnvalue_2 (Class|SlimeObjectif|GetNextAttackPoint _output_get))
    (Variables|Default|SetObjectifLocation _returnvalue_2)
    (Variables|Default|SetCurrentObjectifIsDead false)
    (return)
    (else
      (Development|PrintString "Attention il n'y as pas de Objectif Manager le level" true true "(R=1.000000,G=0.018841,B=0.078564,A=1.000000)"))))

(fn LaunchinDirection
  (params (Direction :type Vector))
  (Variables|Default|SetIsSlimeJumping true)
  (bind _asbp_slime_pawn (Utilities|Casting|CastToBP_SlimePawn (Pawn|GetControlledPawn)))
  (Variables|/Game/BluenPrint/Slime/BP_SlimePawn.BP_SlimePawn_C|SetbIsJumping _asbp_slime_pawn true)
  (Collision|SetCollisionEnabled (Variables|/Game/BluenPrint/Slime/BP_SlimePawn.BP_SlimePawn_C|GetCollision _asbp_slime_pawn) "QueryAndPhysics")
  (Physics|SetSimulatePhysics (Variables|/Game/BluenPrint/Slime/BP_SlimePawn.BP_SlimePawn_C|GetCollision _asbp_slime_pawn) true)
  (Physics|AddImpulse (Variables|/Game/BluenPrint/Slime/BP_SlimePawn.BP_SlimePawn_C|GetCollision _asbp_slime_pawn) (* (Math|Vector|Normalize Direction 0.001) (Variables|Default|GetStartLaunchSpeed)) "None" true)
  (Variables|Default|SetCanStopJump false)
  (Utilities|Time|SetTimerbyFunctionName 0 "SetCanStopJump" 0.1)
  (return))