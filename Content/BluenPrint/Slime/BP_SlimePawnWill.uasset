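; Slime pawn that gives its sphere mesh an animated, colored slime look and nudges other slimes on overlap.
; BeginPlay creates a dynamic material with the set color, then randomizes pulse, noise and band parameters so each instance varies.
; Tick feeds the mesh's reversed forward vector to the material as the slime direction.
; Collision overlaps with exact-class BP_SlimePawn actors offset the other component in XY along the negated, scaled sweep normal.
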(event OnComponentBeginOverlap(Collision)
  (params (OverlappedComponent :type Primitive%20Component%20Object%20Reference) (OtherActor :type Actor%20Object%20Reference) (OtherComp :type Primitive%20Component%20Object%20Reference) (OtherBodyIndex :type Integer) (bFromSweep :type Boolean) (SweepResult :type Hit%20Result%20Structure%20%28by%20ref%29))
  (bind _returnvalue (Math|Conversions|ToVector(Float) -3.0))
  (bind _returnvalue_2 (* (.normal SweepResult) _returnvalue))
  (bind (_x _y) (Math|Vector|BreakVector _returnvalue_2))
  (if (== (Utilities|GetClass OtherActor) "/Game/BluenPrint/Slime/BP_SlimePawn.BP_SlimePawn_C")
    (Transformation|AddWorldOffset OtherComp (Math|Vector|MakeVector _x _y 0.0) false false)))

(event EventBeginPlay
  (bind _returnvalue (Rendering|Material|CreateDynamicMaterialInstance (Variables|Default|GetMaterialParent) "MI_Slimemat" "None" :!class /Script/Engine.KismetMaterialLibrary))
  (Rendering|Material|SetVectorParameterValue _returnvalue "BaseColor" (Variables|Default|GetColor) :!class /Script/Engine.MaterialInstanceDynamic)
  (Rendering|Material|SetMaterial (Variables|Default|GetSphere2) 0 _returnvalue)
  (Rendering|Material|SetScalarParameterValueonMaterials (Variables|Default|GetSphere2) "PulseIntensity" (Math|Random|RandomFloatinRange 1.0 4.0))
  (Rendering|Material|SetScalarParameterValueonMaterials (Variables|Default|GetSphere2) "PulseSpeed" (Math|Random|RandomFloatinRange 1.0 2.0))
  (Rendering|Material|SetVectorParameterValueonMaterials (Variables|Default|GetSphere2) "NoiseWidth" (Math|Vector|MakeVector (Math|Random|RandomFloatinRange 0.0 1.0) (Math|Random|RandomFloatinRange 0.0 1.0) (Math|Random|RandomFloatinRange 0.0 1.0)))
  (Rendering|Material|SetScalarParameterValueonMaterials (Variables|Default|GetSphere2) "BandIntensity" (Math|Random|RandomFloatinRange 1.0 2.0))
  (Rendering|Material|SetScalarParameterValueonMaterials (Variables|Default|GetSphere2) "BandSpeed" (Math|Random|RandomFloatinRange 1.0 2.0)))

(event EventTick
  (params (DeltaSeconds :type Float%20%28single-precision%29))
  (bind _sphere2 (Variables|Default|GetSphere2))
  (Rendering|Material|SetVectorParameterValueonMaterials _sphere2 "SlimeDirection" (* (Math|Vector|GetForwardVector (Transformation|GetWorldRotation _sphere2)) (Math|Conversions|ToVector(Float) -1.0))))

(fn ConstructionScript)