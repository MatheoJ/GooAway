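; Slime objective manager that hands defeat to GM_Pompastronautes when all objectives are dead, and can show end-of-game screens.
; BeginPlay binds OnAllObjectivesDead to a handler that calls the game mode's Lose.
; Separately, while EndTimer is set, Tick waits three seconds, pauses, then calls its own Win or Lose based on WinOrLose.
; Both create their widget once, show the cursor and focus UI input; nothing here sets EndTimer or WinOrLose.
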(event Custom|OnAllObjectivesDead_Event
  (bind _asgm_pompastronautes (Utilities|Casting|CastToGM_Pompastronautes (Game|GetGameMode)))
  (Default|Lose _asgm_pompastronautes))

(event EventBeginPlay
  (EventDispatchers|AssignOnAllObjectivesDead (delegate Custom|OnAllObjectivesDead_Event)))

(event Collision|EventActorBeginOverlap
  (params (OtherActor :type Actor%20Object%20Reference)))

(event EventTick
  (params (DeltaSeconds :type Float%20%28single-precision%29))
  (if (Variables|Default|GetEndTimer)
    (Variables|Default|SetloseTimer (+ DeltaSeconds (Variables|Default|GetloseTimer)))
    (if (> (Variables|Default|GetloseTimer) 3.0)
      (Game|SetGamePaused true)
      (if (Variables|Default|GetWinOrLose)
        (CallFunction|Win)
        (else
          (CallFunction|Lose))))))

(fn ConstructionScript)

(fn Lose
  (if (not (Variables|Default|Getlost))
    (bind _returnvalue (UserInterface|CreateWidget "/Game/Widgets/WB_LoseScreen.WB_LoseScreen_C"))
    (UserInterface|Viewport|AddtoViewport _returnvalue 0)
    (Input|SetInputModeGameandUI (Game|GetPlayerController 0) _returnvalue "DoNotLock" true false)
    (Variables|/Script/Engine.PlayerController|SetbShowMouseCursor (Game|GetPlayerController 0) true)
    (Variables|Default|Setlost true)))

(fn Win
  (if (not (Variables|Default|GetWon))
    (bind _returnvalue (UserInterface|CreateWidget "/Game/Widgets/WB_WinScreen.WB_WinScreen_C"))
    (UserInterface|Viewport|AddtoViewport _returnvalue 0)
    (Input|SetInputModeGameandUI (Game|GetPlayerController 0) _returnvalue "DoNotLock" true false)
    (Variables|/Script/Engine.PlayerController|SetbShowMouseCursor (Game|GetPlayerController 0) true)
    (Variables|Default|SetWon true)))