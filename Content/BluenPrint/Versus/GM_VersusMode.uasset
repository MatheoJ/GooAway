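; Game mode for local two-player versus play that creates the second player and shows a paused win screen for P1 or P2.
; RoomEntry records room start times and drives the HUD and slime spawner, while Tick only advances the timer.
; Helpers handle slime and cryopod totals, leaderboard entries and debug room teleports.
; The room-completion chain (time-up or loss, opening corridors, paychecks) is disconnected and never runs.
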(event Custom|TotalStatAndWin
  (CallFunction|AddLeaderBoardEntrie (Variables|Default|GetTotalMoney) (Variables|Default|GetTotalObjectiveKilled) (Variables|Default|GetTotalObjectivesSaved) (Variables|Default|GetTotalSlimeKilled) "SamSam")
  (bind _returnvalue (UserInterface|CreateWidget "/Game/Widgets/WB_ScoreBoard.WB_ScoreBoard_C"))
  (UserInterface|Viewport|AddtoViewport _returnvalue 0))

(event Custom|ClearLeaderBoard
  (Class|LeaderboardManager|ClearLeaderboard (Subsystems|GetLeaderboardManager)))

(event Custom|P1%20Wins
  (bind _returnvalue (Game|GetPlayerController 0))
  (Development|PrintString "P1Wins!")
  (bind _returnvalue_2 (UserInterface|CreateWidget "/Game/Widgets/VersusMode/WB_WinScreenP1.WB_WinScreenP1_C" _returnvalue))
  (UserInterface|Viewport|AddtoViewport _returnvalue_2 0)
  (Input|SetInputModeGameandUI _returnvalue _returnvalue_2 "DoNotLock" true false)
  (Variables|/Script/Engine.PlayerController|SetbShowMouseCursor (Game|GetPlayerController 0) true)
  (Game|SetGamePaused true))

(event Custom|UnloadLevels
  (Game|UnloadStreamLevel(byName) "Level_0" false)
  (Game|UnloadStreamLevel(byName) "Level_01_Art" false)
  (Game|UnloadStreamLevel(byName) "Level_02_Art" false)
  (Game|UnloadStreamLevel(byName) "Level_03_Art" false)
  (Game|UnloadStreamLevel(byName) "Level_04_Art" false)
  (bind _outactors (Actor|GetAllActorsOfClass "/Game/BluenPrint/Streaming/BP_LoadManager.BP_LoadManager_C"))
  (for _array_element _outactors
    (Default|Reset _array_element)))

(event Custom|P2Wins
  (bind _returnvalue (Game|GetPlayerController 0))
  (Development|PrintString "P2Wins!")
  (bind _returnvalue_2 (UserInterface|CreateWidget "/Game/Widgets/VersusMode/WB_WinScreenP2.WB_WinScreenP2_C" _returnvalue))
  (UserInterface|Viewport|AddtoViewport _returnvalue_2 0)
  (Input|SetInputModeGameandUI _returnvalue _returnvalue_2 "DoNotLock" true false)
  (Variables|/Script/Engine.PlayerController|SetbShowMouseCursor (Game|GetPlayerController 0) true)
  (Game|SetGamePaused true))

(event EventBeginPlay
  (if (< (Class|GameplayStatics|GetNumLocalPlayerControllers) 2)
    (Class|GameplayStatics|CreatePlayer -1))
  (Audio|Components|Audio|Stop (Variables|Default|GetRoomFinishedSound))
  (Utilities|FlowControl|Delay 1.0)
  (bind _foundwidgets (Widget|GetAllWidgetsOfClass "/Game/Widgets/New_HUD/WB_HUDBothPlayers.WB_HUDBothPlayers_C" true))
  (bind _output_get (Variables|Default|SetHUD (Utilities|Array|Get(acopy) _foundwidgets)))
  (Default|HideTimer _output_get)
  (Utilities|FlowControl|Delay 1.0))

(event EventTick
  (params (DeltaSeconds :type Float%20%28single-precision%29))
  (CallFunction|UpdateTimer DeltaSeconds))

(fn ConstructionScript)

(fn UpdateTimer
  (params (DeltaTime :type Float%20%28double-precision%29))
  (Variables|Default|SetTimer (+ DeltaTime (Variables|Default|GetTimer))))

(fn Lose
  (Variables|Default|Setlost true))

(fn Win
  (if (not (Variables|Default|GetWon))
    (bind _returnvalue (UserInterface|CreateWidget "/Game/Widgets/WB_WinScreen.WB_WinScreen_C"))
    (UserInterface|Viewport|AddtoViewport _returnvalue 0)
    (Input|SetInputModeGameandUI (Game|GetPlayerController 0) _returnvalue "DoNotLock" true false)
    (Variables|/Script/Engine.PlayerController|SetbShowMouseCursor (Game|GetPlayerController 0) true)
    (Variables|Default|SetWon true)))

(fn RoomEntry
  (params (Room :type E_Room%20Enum :default "NewEnumerator0"))
  (bind _timer (Variables|Default|GetTimer))
  (Development|PrintString (Utilities|String|Append "Entered : " (Utilities|String|EnumtoString Room)))
  (bind _output_get (Variables|Default|SetCurrentRoom Room))
  (switch Utilities|FlowControl|Switch|SwitchonE_Room _output_get
    (:NewEnumerator0
      (Variables|Default|SetLevel1EntryTime _timer)
      (Default|StartVideo (Variables|Default|GetHUD)))
    (:NewEnumerator1
      (Variables|Default|SetLevel2EntryTime _timer)
      (Default|ShowTimer (Variables|Default|GetHUD))
      (bind _returnvalue (Actor|GetActorOfClass "/Game/BluenPrint/BP_SpawnerManager.BP_SpawnerManager_C"))
      (Class|SpawnerManager|BeginSpawning _returnvalue))
    (:NewEnumerator2
      (Variables|Default|SetLevel3EntryTime _timer)
      (Default|ShowTimer (Variables|Default|GetHUD))
      (bind _returnvalue_2 (Actor|GetActorOfClass "/Game/BluenPrint/BP_SpawnerManager.BP_SpawnerManager_C"))
      (Class|SpawnerManager|BeginSpawning _returnvalue_2))
    (:NewEnumerator3
      (Variables|Default|SetLevel4EntryTime _timer)
      (Default|ShowTimer (Variables|Default|GetHUD))
      (bind _returnvalue_3 (Actor|GetActorOfClass "/Game/BluenPrint/BP_SpawnerManager.BP_SpawnerManager_C"))
      (Class|SpawnerManager|BeginSpawning _returnvalue_3))))

(fn Time'sUpCheck
  (params (entry%20time :type Float%20%28double-precision%29) (total%20time :type Float%20%28double-precision%29))
  (bind _timer (Variables|Default|GetTimer))
  (bind _returnvalue (- _timer entry%20time))
  (bind _output_get (Variables|Default|SetCurrentRemainingTime (Math|Float|Max(Float) (- total%20time _returnvalue) 0.0)))
  (Variables|/Game/Widgets/New_HUD/WB_HUDBothPlayers.WB_HUDBothPlayers_C|SetTimeLeftOnLevel (Variables|Default|GetHUD) _output_get)
  (return (> _returnvalue total%20time)))

(fn PresenceJoueurs
  (bind _output_get (Variables|Default|SetLastID (+ (Variables|Default|GetLastID) 1)))
  (return (- 1 _output_get)))

(fn GetObjectifStats
  (LocalVariables|SetDeadNum 0)
  (LocalVariables|SetAliveNum 0)
  (bind _outactors (Actor|GetAllActorsOfClass "/Game/BluenPrint/BP_Cryopods.BP_Cryopods_C"))
  (for _array_element _outactors
    (if (Variables|/Script/Pompastronautes.SlimeObjectif|GetbIsDead _array_element)
      (LocalVariables|SetDeadNum (+ (LocalVariables|GetDeadNum) 1))
      (else
        (LocalVariables|SetAliveNum (+ (LocalVariables|GetAliveNum) 1)))))
  (return (LocalVariables|GetDeadNum) (LocalVariables|GetAliveNum)))

(fn GetKilledSlime
  (LocalVariables|SetTotalSlimeSpawned 0)
  (bind _outactors (Actor|GetAllActorsOfClass "/Game/BluenPrint/BP_SpawnerWave.BP_SpawnerWave_C"))
  (for _array_element _outactors
    (bind _asbp_spawner_wave (Utilities|Casting|CastToBP_SpawnerWave _array_element))
    (LocalVariables|SetTotalSlimeSpawned (+ (Variables|/Script/Pompastronautes.SpawnerWave|GetTotalSlimesSpawned _asbp_spawner_wave) (LocalVariables|GetTotalSlimeSpawned))))
  (bind _outactors_2 (Actor|GetAllActorsOfClass "/Game/BluenPrint/Slime/BP_SlimePawn.BP_SlimePawn_C"))
  (return (- (LocalVariables|GetTotalSlimeSpawned) (Utilities|Array|Length _outactors_2))))

(fn LightGreenHouseSign
  (bind _returnvalue (Actor|GetActorOfClass "/Game/Art/Assets/SortieGreenhouse.SortieGreenhouse_C"))
  (Default|TurnGreen _returnvalue))

(fn GetLeaderBoardEntries
  (params (ByMoney :type Boolean) (BySlimes :type Boolean) (ByObjectivesSaved :type Boolean) (Descending :type Boolean))
  (return (Class|LeaderboardManager|GetSortedLeaderboard (Subsystems|GetLeaderboardManager) ByMoney BySlimes ByObjectivesSaved Descending)))

(fn AddLeaderBoardEntrie
  (params (Money :type Integer) (ObjectivesKilled :type Integer) (Objtectives :type Integer) (NumSlimeKilled :type Integer) (Name :type String))
  (Class|LeaderboardManager|AddLeaderboardEntry (Subsystems|GetLeaderboardManager) Name Money NumSlimeKilled Objtectives ObjectivesKilled))

(fn ResetTotalStats
  (Variables|Default|SetTotalMoney 0)
  (Variables|Default|SetTotalObjectiveKilled 0)
  (Variables|Default|SetTotalObjectivesSaved 0)
  (Variables|Default|SetTotalSlimeKilled 0))

(fn UpdateTotalStats
  (bind _killedslimes (CallFunction|GetKilledSlime))
  (Variables|Default|SetTotalSlimeKilled (+ _killedslimes (Variables|Default|GetTotalSlimeKilled)))
  (bind (_deadobjectifsnumber _aliveobjectifnumber) (CallFunction|GetObjectifStats))
  (Variables|Default|SetTotalObjectivesSaved (+ _aliveobjectifnumber (Variables|Default|GetTotalObjectivesSaved)))
  (Variables|Default|SetTotalObjectiveKilled (+ _deadobjectifsnumber (Variables|Default|GetTotalObjectiveKilled))))

(fn DebugLoadLevel2
  (Default|HideTimer (Variables|Default|GetHUD))
  (Variables|Default|SetCurrentRoom "NewEnumerator5")
  (CallFunction|UnloadLevels)
  (bind _outactors (Actor|GetAllActorsOfClass "/Game/ThirdPerson/Blueprints/BP_ThirdPersonCharacter_onlyBP.BP_ThirdPersonCharacter_onlyBP_C"))
  (for _array_element _outactors
    (Transformation|SetActorLocation _array_element "1250.000000,3160.000000,200.000000" false false)))

(fn DebugLoadLevel3
  (Default|HideTimer (Variables|Default|GetHUD))
  (Variables|Default|SetCurrentRoom "NewEnumerator6")
  (CallFunction|UnloadLevels)
  (bind _outactors (Actor|GetAllActorsOfClass "/Game/ThirdPerson/Blueprints/BP_ThirdPersonCharacter_onlyBP.BP_ThirdPersonCharacter_onlyBP_C"))
  (for _array_element _outactors
    (Transformation|SetActorLocation _array_element "1210.000000,8740.000000,160.000000" false false)))

(fn DebugLoadLevel4
  (Default|HideTimer (Variables|Default|GetHUD))
  (Variables|Default|SetCurrentRoom "NewEnumerator7")
  (CallFunction|UnloadLevels)
  (bind _outactors (Actor|GetAllActorsOfClass "/Game/ThirdPerson/Blueprints/BP_ThirdPersonCharacter_onlyBP.BP_ThirdPersonCharacter_onlyBP_C"))
  (for _array_element _outactors
    (Transformation|SetActorLocation _array_element "-3525.000000,10010.000000,160.000000" false false)))