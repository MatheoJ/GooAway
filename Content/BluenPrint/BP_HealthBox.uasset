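; BP_HealthBox is a visual health gauge for an objective, driven by life-update and death events.
; LifeIsUpdated shrinks the Pivot's Z scale as life drops, using a clamped range remap and Lerp.
; The first drop below full life also enables custom depth rendering on the box and plane meshes through a DoOnce.
; ObjectiveDead turns that custom depth off again.
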(event EventBeginPlay)

(event Collision|EventActorBeginOverlap
  (params (OtherActor :type Actor%20Object%20Reference)))

(event EventTick
  (params (DeltaSeconds :type Float%20%28single-precision%29)))

(event EventLifeIsUpdated
  (params (CurrentLife :type Float%20%28double-precision%29) (fish :type Child%20Actor%20Component%20Object%20Reference))
  (bind _pivot (Variables|Default|GetPivot))
  (bind _relativescale3d (Variables|/Script/Engine.SceneComponent|GetRelativeScale3D _pivot))
  (Utilities|FlowControl|Sequence
    (:then_0
      (if (< CurrentLife 1e+02)
        (Utilities|FlowControl|DoOnce false
          (:Completed
            (Rendering|SetRenderCustomDepth (Variables|Default|GetSM_Boxe_objectif) true)
            (Rendering|SetRenderCustomDepth (Variables|Default|GetSM_PlaneAdri1) true)))))
    (:then_1
      (Transformation|SetRelativeScale3D _pivot (Math|Vector|MakeVector (.x _relativescale3d) (.y _relativescale3d) (Math|Float|Lerp 1.0 0.0 (Math|Float|MapRangeClamped CurrentLife 1e+02 0.0 0.0 1.0)))))))

(event EventObjectiveDead
  (Rendering|SetRenderCustomDepth (Variables|Default|GetSM_Boxe_objectif) false)
  (Rendering|SetRenderCustomDepth (Variables|Default|GetSM_PlaneAdri1) false))

(fn ConstructionScript)