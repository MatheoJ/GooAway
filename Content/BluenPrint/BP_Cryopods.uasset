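; Cryopod objective that shows its remaining life and can be highlighted as a lock target.
; As life drops, a dynamic glass material cracks, bubbles shrink, and a timeline-driven white-to-red light pulses faster with a louder, higher warning sound.
; Life and death are messaged to child actors; death also plays an explosion sound, starts smoke and disables custom depth.
; Lock events toggle a fresnel glow tinted green to red by life.
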(event Custom|Construct
  (bind _currentlife (Variables|Default|GetCurrentLife))
  (bind _returnvalue (Math|Float|MapRangeClamped _currentlife 1e+02 0.0 0.0 1.0))
  (Class|BPIInterface|LifeIsUpdated(Message) (Actor|GetAllChildActors true) (Variables|Default|GetCurrentLife))
  (bind _returnvalue_2 (Rendering|Material|CreateDynamicMaterialInstance "/Game/Material/MI_Healt_Vitre_InstBrisable.MI_Healt_Vitre_InstBrisable" "None" "None" :!class /Script/Engine.KismetMaterialLibrary))
  (bind _output_get (Variables|Default|SetM_Brise _returnvalue_2))
  (Rendering|Material|SetMaterial (Variables|Default|GetCube) 0 _output_get)
  (Rendering|Material|SetScalarParameterValue (Variables|Default|GetM_Brise) "Refract" (Math|Float|Lerp 0.0 (Variables|Default|GetCracks) _returnvalue) :!class /Script/Engine.MaterialInstanceDynamic)
  (if (< _currentlife 1.0)
    (Class|SlimeObjectif|OnDeath)
    (else
      (|LightTimer_2_2_2_2 (Variables|Default|GetTimeline_0) _returnvalue 2.0
        (:then2
          (CallFunction|Play3DSound _returnvalue (Variables|Default|GetwarningSound) 0.05 2.0)
          (Class|NiagaraComponent|SetPaused (Variables|Default|GetNS_Fumee1) true)
          (Class|NiagaraComponent|SetPaused (Variables|Default|GetNS_Fumee) true))))))

(event EventBeginPlay
  (bind _currentlife (Variables|Default|GetCurrentLife))
  (bind _returnvalue (Math|Float|MapRangeClamped _currentlife 1e+02 0.0 0.0 1.0))
  (bind _returnvalue_2 (Rendering|Material|CreateDynamicMaterialInstance "/Game/Art/MaterialInstances/MI_Objectif.MI_Objectif" "None" "None" :!class /Script/Engine.KismetMaterialLibrary))
  (bind _output_get (Variables|Default|SetM_obj _returnvalue_2))
  (Rendering|Material|SetMaterial (Variables|Default|GetCube) 1 _output_get)
  (Class|BPIInterface|LifeIsUpdated(Message) (Actor|GetAllChildActors true) (Variables|Default|GetCurrentLife))
  (bind _returnvalue_3 (Rendering|Material|CreateDynamicMaterialInstance "/Game/Material/MI_Healt_Vitre_InstBrisable.MI_Healt_Vitre_InstBrisable" "None" "None" :!class /Script/Engine.KismetMaterialLibrary))
  (bind _output_get_2 (Variables|Default|SetM_Brise _returnvalue_3))
  (Rendering|Material|SetMaterial (Variables|Default|GetCube) 0 _output_get_2)
  (Rendering|Material|SetScalarParameterValue (Variables|Default|GetM_Brise) "Refract" (Math|Float|Lerp 0.0 (Variables|Default|GetCracks) _returnvalue) :!class /Script/Engine.MaterialInstanceDynamic)
  (if (< _currentlife 1.0)
    (Class|SlimeObjectif|OnDeath)
    (else
      (|LightTimer_2_2_2_2 (Variables|Default|GetTimeline_0) _returnvalue 2.0
        (:then2
          (CallFunction|Play3DSound _returnvalue (Variables|Default|GetwarningSound) 0.05 2.0)
          (Class|NiagaraComponent|SetPaused (Variables|Default|GetNS_Fumee1) true)
          (Class|NiagaraComponent|SetPaused (Variables|Default|GetNS_Fumee) true))))))

(event Collision|EventActorBeginOverlap
  (params (OtherActor :type Actor%20Object%20Reference)))

(event EventTick
  (params (DeltaSeconds :type Float%20%28single-precision%29)))

(event EventOnLifeUpdated
  (bind _currentlife (Variables|Default|GetCurrentLife))
  (bind _returnvalue (Math|Float|MapRangeClamped _currentlife 1e+02 0.0 0.0 1.0))
  (if (not (Variables|Default|GetbDead))
    (Class|BPIInterface|LifeIsUpdated(Message) (Actor|GetAllChildActors true) (Variables|Default|GetCurrentLife) (Variables|Default|GetBP_Fishes))
    (Rendering|Material|SetScalarParameterValue (Variables|Default|GetM_Brise) "Refract" (Math|Float|Lerp 0.0 (Variables|Default|GetCracks) _returnvalue) :!class /Script/Engine.MaterialInstanceDynamic)
    (|LightTimer_2_2_2 (Variables|Default|GetTimeline) _returnvalue 2.0
      (:then
        (CallFunction|Play3DSound _returnvalue (Variables|Default|GetwarningSound) 0.02 2.0)
        (Niagara|SetNiagaraVariable(Float) (Variables|Default|GetNS_Bubbles) "Scale" (Math|Float|Lerp 3.0 0.0 _returnvalue))))))

(event EventOnDeath
  (Class|BPIInterface|ObjectiveDead(Message) (Actor|GetAllChildActors true))
  (Rendering|SetRenderCustomDepth (Variables|Default|GetCube) false)
  (Variables|Default|SetbDead true)
  (CallFunction|Play3DSound 1.0 (Variables|Default|GetExploSound) 4.0 1.0)
  (Components|Activation|Deactivate (Variables|Default|GetNS_Bubbles))
  (Components|Activation|Activate (Variables|Default|GetNS_Fumee1) false)
  (Components|Activation|Activate (Variables|Default|GetNS_Fumee) false))

(event EventIsLockable
  (bind _m_obj (Variables|Default|GetM_obj))
  (Rendering|Material|SetVectorParameterValue _m_obj "colorEmi" (Math|Color|Lerp(LinearColor) "(R=0.000000,G=1.000000,B=0.121732,A=1.000000)" "(R=1.000000,G=0.000000,B=0.008376,A=1.000000)" (Math|Float|MapRangeClamped (Variables|Default|GetCurrentLife) 1e+02 0.0 0.0 1.0)) :!class /Script/Engine.MaterialInstanceDynamic)
  (Rendering|Material|SetScalarParameterValue _m_obj "emissiveFresnel" 1.0 :!class /Script/Engine.MaterialInstanceDynamic))

(event EventDelock
  (Rendering|Material|SetScalarParameterValue (Variables|Default|GetM_obj) "emissiveFresnel" 0.0 :!class /Script/Engine.MaterialInstanceDynamic))

(fn ConstructionScript
  (CallFunction|Construct))

(fn Play3DSound
  (params (Alpha :type Float%20%28double-precision%29) (Sound :type Audio%20Component%20Object%20Reference) (Volume :type Float%20%28double-precision%29) (Pitch :type Float%20%28double-precision%29))
  (Audio|Components|Audio|SetVolumeMultiplier Sound (Math|Float|Lerp 0.0 Volume Alpha) :!class /Script/Engine.AudioComponent)
  (Audio|Components|Audio|SetPitchMultiplier Sound (Math|Float|Lerp 0.0 Pitch Alpha))
  (Audio|Components|Audio|Play Sound 1.0))