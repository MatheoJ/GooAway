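; BP_DummySlime is a slime dummy actor, stored among outdated gun Blueprints, that can be launched to fly in a straight line.
; Fly stores a normalized direction and sets IsFlying.
; While that flag is set, Tick moves the actor along the direction at FlyingSpeed without sweeping and spins it in local pitch at RotationSpeed.
; Nothing in its graphs stops the flight or handles hits.
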(event EventBeginPlay)

(event Collision|EventActorBeginOverlap
  (params (OtherActor :type Actor%20Object%20Reference)))

(event EventTick
  (params (DeltaSeconds :type Float%20%28single-precision%29))
  (if (Variables|Default|GetIsFlying)
    (Transformation|AddActorWorldOffset (* (Variables|Default|GetFlyDirection) (* DeltaSeconds (Variables|Default|GetFlyingSpeed))))
    (Transformation|AddActorLocalRotation (Math|Rotator|MakeRotator 0.0 (* DeltaSeconds (Variables|Default|GetRotationSpeed)) 0.0) false false)))

(fn ConstructionScript)

(fn Fly
  (params (direction :type Vector))
  (Variables|Default|SetIsFlying true)
  (Variables|Default|SetFlyDirection (Math|Vector|Normalize direction)))