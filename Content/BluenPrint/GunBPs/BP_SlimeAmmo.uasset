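; BP_SlimeAmmo is a slime gun projectile that passes its AmmoType to any SlimeBase it strikes through OnHitBySlime.
; Fly launches it along a given direction at fixed speed, and Tick restores gravity once MaxFlyingTime elapses so the shot starts to drop.
; Sphere1 overlaps notify slimes, while hits and overlaps on either sphere destroy the projectile, except overlaps with other slime ammo.
; Debug prints remain in the collision handlers.
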(event OnComponentBeginOverlap(Sphere1)
  (params (OverlappedComponent :type Primitive%20Component%20Object%20Reference) (OtherActor :type Actor%20Object%20Reference) (OtherComp :type Primitive%20Component%20Object%20Reference) (OtherBodyIndex :type Integer) (bFromSweep :type Boolean) (SweepResult :type Hit%20Result%20Structure%20%28by%20ref%29))
  (Development|PrintString (Utilities|GetDisplayName OtherActor) true true "(R=1.000000,G=0.000000,B=0.145770,A=1.000000)")
  (bind _asslime_base (Utilities|Casting|CastToSlimeBase OtherActor)
    (:then
      (Class|SlimeBase|OnHitbySlime _asslime_base (Variables|Default|GetAmmoType))
      (Actor|DestroyActor))
    (:CastFailed
      (Utilities|Casting|CastToBP_SlimeAmmo OtherActor
        (:CastFailed
          (Actor|DestroyActor))))))

(event OnComponentHit(Sphere1)
  (params (HitComponent :type Primitive%20Component%20Object%20Reference) (OtherActor :type Actor%20Object%20Reference) (OtherComp :type Primitive%20Component%20Object%20Reference) (NormalImpulse :type Vector :default "0, 0, 0") (Hit :type Hit%20Result%20Structure%20%28by%20ref%29))
  (Actor|DestroyActor)
  (Development|PrintString "Hello"))

(event OnComponentHit(Sphere)
  (params (HitComponent :type Primitive%20Component%20Object%20Reference) (OtherActor :type Actor%20Object%20Reference) (OtherComp :type Primitive%20Component%20Object%20Reference) (NormalImpulse :type Vector :default "0, 0, 0") (Hit :type Hit%20Result%20Structure%20%28by%20ref%29))
  (Actor|DestroyActor))

(event OnComponentBeginOverlap(Sphere)
  (params (OverlappedComponent :type Primitive%20Component%20Object%20Reference) (OtherActor :type Actor%20Object%20Reference) (OtherComp :type Primitive%20Component%20Object%20Reference) (OtherBodyIndex :type Integer) (bFromSweep :type Boolean) (SweepResult :type Hit%20Result%20Structure%20%28by%20ref%29))
  (Utilities|Casting|CastToBP_SlimeAmmo OtherActor
    (:CastFailed
      (Development|PrintString (Utilities|GetDisplayName OtherActor) true true "(R=1.000000,G=0.111332,B=0.000000,A=1.000000)")
      (Actor|DestroyActor))))

(event EventBeginPlay)

(event Collision|EventActorBeginOverlap
  (params (OtherActor :type Actor%20Object%20Reference)))

(event EventTick
  (params (DeltaSeconds :type Float%20%28single-precision%29))
  (if (Variables|Default|GetIsFlying)
    (Variables|Default|SetFlyingTime (+ (Variables|Default|GetFlyingTime) DeltaSeconds))
    (if (not (< (Variables|Default|GetFlyingTime) (Variables|Default|GetmaxFlyingTime)))
      (Variables|Default|SetIsFlying false)
      (Variables|/Script/Engine.ProjectileMovementComponent|SetProjectileGravityScale (Variables|Default|GetProjectileMovement) 1.0))))

(event Collision|EventHit
  (params (MyComp :type Primitive%20Component%20Object%20Reference) (Other :type Actor%20Object%20Reference) (OtherComp :type Primitive%20Component%20Object%20Reference) (bSelfMoved :type Boolean) (HitLocation :type Vector :default "0, 0, 0") (HitNormal :type Vector :default "0, 0, 0") (NormalImpulse :type Vector :default "0, 0, 0") (Hit :type Hit%20Result%20Structure%20%28by%20ref%29))
  (Actor|DestroyActor))

(fn ConstructionScript)

(fn Fly
  (params (direction :type Vector))
  (bind _output_get (Variables|Default|SetFlyDirection (Math|Vector|Normalize direction)))
  (Game|Components|ProjectileMovement|SetVelocityinLocalSpace (Variables|Default|GetProjectileMovement) (* (Math|Transform|InverseTransformDirection (Transformation|GetActorTransform) _output_get) 1000))
  (Variables|Default|SetIsFlying true))