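; BP_Ammo is an ammo projectile actor that destroys itself when its Cube component registers a hit.
; FlyPhysics launches the physics-simulated Cube with an impulse along the given direction and a spin torque.
; Tick times the flight, then turns on physics and gravity once the maximum flying time is reached.
; The alternative Fly only stores a direction and disables physics, as its manual movement code is disconnected and marked outdated.
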(event OnComponentHit(Cube)
  (params (HitComponent :type Primitive%20Component%20Object%20Reference) (OtherActor :type Actor%20Object%20Reference) (OtherComp :type Primitive%20Component%20Object%20Reference) (NormalImpulse :type Vector :default "0, 0, 0") (Hit :type Hit%20Result%20Structure%20%28by%20ref%29))
  (Actor|DestroyActor))

(event OnComponentHit(Sphere)
  (params (HitComponent :type Primitive%20Component%20Object%20Reference) (OtherActor :type Actor%20Object%20Reference) (OtherComp :type Primitive%20Component%20Object%20Reference) (NormalImpulse :type Vector :default "0, 0, 0") (Hit :type Hit%20Result%20Structure%20%28by%20ref%29)))

(event OnComponentBeginOverlap(Sphere)
  (params (OverlappedComponent :type Primitive%20Component%20Object%20Reference) (OtherActor :type Actor%20Object%20Reference) (OtherComp :type Primitive%20Component%20Object%20Reference) (OtherBodyIndex :type Integer) (bFromSweep :type Boolean) (SweepResult :type Hit%20Result%20Structure%20%28by%20ref%29)))

(event EventBeginPlay
  (Collision|SetActorEnableCollision true)
  (Collision|SetCollisionEnabled (Variables|Default|GetCube) "QueryAndPhysics"))

(event Collision|EventActorBeginOverlap
  (params (OtherActor :type Actor%20Object%20Reference)))

(event EventTick
  (params (DeltaSeconds :type Float%20%28single-precision%29))
  (if (Variables|Default|GetIsFlying)
    (Variables|Default|SetFlyingTime (+ (Variables|Default|GetFlyingTime) DeltaSeconds))
    (if (not (< (Variables|Default|GetFlyingTime) (Variables|Default|GetmaxFlyingTime)))
      (Variables|Default|SetIsFlying false)
      (Physics|SetSimulatePhysics (Variables|Default|GetCube) true)
      (Physics|SetEnableGravity (Variables|Default|GetCube) true))))

(event Collision|EventHit
  (params (MyComp :type Primitive%20Component%20Object%20Reference) (Other :type Actor%20Object%20Reference) (OtherComp :type Primitive%20Component%20Object%20Reference) (bSelfMoved :type Boolean) (HitLocation :type Vector :default "0, 0, 0") (HitNormal :type Vector :default "0, 0, 0") (NormalImpulse :type Vector :default "0, 0, 0") (Hit :type Hit%20Result%20Structure%20%28by%20ref%29)))

(fn ConstructionScript)

(fn Fly
  (params (direction :type Vector))
  (Variables|Default|SetIsFlying true)
  (Variables|Default|SetFlyDirection (Math|Vector|Normalize direction))
  (Physics|SetSimulatePhysics (Variables|Default|GetCube) false))

(fn FlyPhysics
  (params (Direction :type Vector) (Rotation :type Vector))
  (Variables|Default|SetIsFlying true)
  (Physics|SetSimulatePhysics (Variables|Default|GetCube) true)
  (Physics|AddImpulse (Variables|Default|GetCube) (* (Math|Vector|Normalize Direction) 150) "None" false)
  (Class|PrimitiveComponent|AddTorqueinRadians (Variables|Default|GetCube) (* Rotation 300) "None" true))

(fn Tests)